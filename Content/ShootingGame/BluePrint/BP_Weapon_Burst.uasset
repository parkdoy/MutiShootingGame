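; Burst-fire weapon Blueprint that overrides its parent's trigger and follow-up shot logic.
; PullTrigger runs the parent logic and queues three additional shots, while the empty ReleaseTrigger override leaves the burst uninterrupted on release.
; AddtionalShot, a timer callback not started here, plays the rifle shoot montage, decrements ammo and shot count, updates the HUD, and clears its timer when either runs out.
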(fn ConstructionScript
  (|CallParentFunction))

(fn PullTrigger
  (params (charactor :type Character%20Object%20Reference))
  (|CallParentFunction charactor)
  (Variables|Default|SetAddshotCnt 3))

(fn ReleaseTrigger)

(fn AddtionalShot
  (bind _owncharater (Variables|Default|GetOwnCharater))
  (Utilities|IsValid _owncharater
    (:Is%20Valid
      (if (and (> (Variables|Default|GetAmmo) 0) (> (Variables|Default|GetAddshotCnt) 0))
        (Animation|PlayAnimMontage _owncharater "/Game/RifleAnimsetPro/Animations/Rifle_ShootOnce_Montage.Rifle_ShootOnce_Montage" 1.0 "None")
        (Math|Integer|DecrementInt (Variables|Default|GetAmmo)
          (:%20%20
            (Math|Integer|DecrementInt (Variables|Default|GetAddshotCnt)
              (:%20%20
                (bind _asmy_hud (Utilities|Casting|CastToMyHUD (HUD|GetHUD (Game|GetPlayerController 0))))
                (Variables|/Game/ShootingGame/Widget/ShootingHUDwidget.ShootingHUDwidget_C|SetText_Ammo (Variables|/Game/ShootingGame/GameMode/MyHUD.MyHUD_C|GetHUDWidget _asmy_hud) (Utilities|Text|ToText(Integer) (Variables|Default|GetAmmo)))))))
        (else
          (Utilities|Time|ClearTimerbyFunctionName 0 "AddtionalShot"))))))