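; BP_Weapon is a rifle that a BP_ShootingCharater equips through EventPress, dropping any weapon it already holds.
; Attaching snaps it to the "weapon" socket; detaching restores physics.
; PullTrigger loops a timer that replays the character's fire montage until ReleaseTrigger or the owner becomes invalid.
; EventNotifyFire separately spends ammo, spawns muzzle effects, plays audio and updates the HUD counter.
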(event EventBeginPlay)

(event Collision|EventActorBeginOverlap
  (params (OtherActor :type Actor%20Object%20Reference)))

(event EventTick
  (params (DeltaSeconds :type Float%20%28single-precision%29)))

(fn ConstructionScript)

(fn AttachtoCharacter
  (params (character :type Character%20Object%20Reference))
  (bind _staticmesh (Variables|Default|GetStaticMesh))
  (Physics|SetSimulatePhysics _staticmesh false)
  (Collision|SetCollisionEnabled _staticmesh "QueryAndPhysics")
  ;[1 1 1] 부모는 케릭터 타깃은 총
  (Transformation|AttachComponentToComponent (Variables|/Script/Engine.Character|GetMesh character) "weapon" "SnapToTarget" "SnapToTarget" "KeepWorld" true)
  (bind _asbp_shooting_charater (Utilities|Casting|CastToBP_ShootingCharater character))
  (bind _output_get (Variables|Default|SetOwnCharater _asbp_shooting_charater))
  (Variables|/Game/ShootingGame/GameMode/BP_ShootingCharater.BP_ShootingCharater_C|SetAttached%20Weapon _output_get self)
  (CallFunction|UpdateUI (Variables|Default|GetAmmo)))

(fn DetachtoCharacter
  (params (Character :type Character%20Object%20Reference))
  (bind _staticmesh (Variables|Default|GetStaticMesh))
  (Transformation|DetachFromActor "KeepWorld" "KeepWorld" "KeepWorld")
  (Collision|SetCollisionEnabled _staticmesh "QueryAndPhysics")
  (Physics|SetSimulatePhysics _staticmesh true)
  (bind _asbp_shooting_charater (Utilities|Casting|CastToBP_ShootingCharater Character))
  (Variables|/Game/ShootingGame/GameMode/BP_ShootingCharater.BP_ShootingCharater_C|SetAttached%20Weapon _asbp_shooting_charater 0)
  (CallFunction|UpdateUI))

(fn PullTrigger
  (params (charactor :type Character%20Object%20Reference))
  (Utilities|Time|SetTimerbyFunctionName 0 "AddtionalShot" 0.1 true))

(fn EventNotifyFire
  (bind _staticmesh (Variables|Default|GetStaticMesh))
  (bind _isusedammo (CallFunction|UseAmmo))
  (if _isusedammo
    (Effects|SpawnEmitteratLocation "/Game/StarterContent/Particles/P_Explosion.P_Explosion" (Transformation|GetSocketLocation _staticmesh "Muzzle") (Transformation|GetSocketRotation _staticmesh "Muzzle") "0.150000,0.150000,0.150000")
    (Audio|Components|Audio|Play (Variables|Default|GetAudio) 0.0)))

(fn AddtionalShot
  (bind _owncharater (Variables|Default|GetOwnCharater))
  (Utilities|IsValid _owncharater
    (:Is%20Valid
      (Animation|PlayAnimMontage _owncharater "/Game/RifleAnimsetPro/Animations/Rifle_ShootOnce_Montage.Rifle_ShootOnce_Montage" 1.0 "None"))
    (:Is%20Not%20Valid
      (Utilities|Time|ClearTimerbyFunctionName 0 "AddtionalShot"))))

(fn ReleaseTrigger
  (Utilities|Time|ClearTimerbyFunctionName 0 "AddtionalShot"))

(fn UpdateUI
  (params (Ammo :type Integer))
  (bind _asmy_hud (Utilities|Casting|CastToMyHUD (HUD|GetHUD (Game|GetPlayerController 0))))
  (Default|UpdateAmmo _asmy_hud Ammo))

(fn UseAmmo
  (bind _ammo (Variables|Default|GetAmmo))
  (if (> _ammo 0)
    (bind _result (Math|Integer|DecrementInt _ammo)
      (:%20%20
        (CallFunction|UpdateUI _result)
        (return true)))
    (else
      (return false))))

(fn SetAmmo
  (params (Ammo :type Integer))
  (bind _output_get (Variables|Default|SetAmmo Ammo))
  (CallFunction|UpdateUI _output_get))

(fn EventPress
  (params (character :type Character%20Object%20Reference))
  (bind _asbp_shooting_charater (Utilities|Casting|CastToBP_ShootingCharater character))
  (Utilities|IsValid (Variables|/Game/ShootingGame/GameMode/BP_ShootingCharater.BP_ShootingCharater_C|GetAttached%20Weapon _asbp_shooting_charater)
    (:Is%20Valid
      (CallFunction|DetachtoCharacter (Variables|/Game/ShootingGame/GameMode/BP_ShootingCharater.BP_ShootingCharater_C|GetAttached%20Weapon _asbp_shooting_charater) character))
    (:Is%20Not%20Valid
      _))
  (CallFunction|AttachtoCharacter character)
  (return true))

(fn EventRelease
  (params (character :type Character%20Object%20Reference))
  (return false))